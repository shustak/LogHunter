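; Teleporter actor that moves LogHunterCharacter actors entering its portal mesh to a linked DestinationTeleporter.
; On overlap it calls IncomingTeleport on the destination, which shifts the character by the offset between the two teleporters, keeping its relative position.
; The receiver tracks arrivals in IncomingActors until their overlap ends, preventing immediate bounce-back.
; The construction script clears self-links and tints a dynamic portal material with Color, or grey when unlinked.
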(event OnComponentBeginOverlap(PortalMesh)
  (params (OverlappedComponent :type Primitive%20Component%20Object%20Reference) (OtherActor :type Actor%20Object%20Reference) (OtherComp :type Primitive%20Component%20Object%20Reference) (OtherBodyIndex :type Integer) (bFromSweep :type Boolean) (SweepResult :type Hit%20Result%20Structure%20%28by%20ref%29))
  (if (CallFunction|CanActorTeleport OtherActor)
    (bind _destinationteleporter (Variables|Default|GetDestinationTeleporter)
      (:then
        (CallFunction|IncomingTeleport _destinationteleporter OtherActor self))
      (:else))))

(event OnComponentEndOverlap(PortalMesh)
  (params (OverlappedComponent :type Primitive%20Component%20Object%20Reference) (OtherActor :type Actor%20Object%20Reference) (OtherComp :type Primitive%20Component%20Object%20Reference) (OtherBodyIndex :type Integer))
  (Utilities|Array|RemoveItem (Variables|Default|GetIncomingActors) OtherActor))

(event Custom|IncomingTeleport
  (params (incomingActor :type Actor%20Object%20Reference) (InvokingTeleport :type Teleporter%20BP%20Object%20Reference))
  (CallFunction|HandleIncomingTeleport incomingActor InvokingTeleport))

(fn ConstructionScript
  (if (== (Variables|Default|GetDestinationTeleporter) self)
    (Variables|Default|SetDestinationTeleporter 0))
  (bind _returnvalue (Rendering|Material|CreateDynamicMaterialInstance "/Game/Blueprints/M_Teleporter.M_Teleporter" "None" "None" :!class /Script/Engine.KismetMaterialLibrary))
  (bind _output_get (LocalVariables|SetMaterialInstance _returnvalue))
  (Rendering|Material|SetMaterial (Variables|Default|GetPortalMesh) 0 _output_get)
  (Rendering|Material|SetVectorParameterValue (LocalVariables|GetMaterialInstance) "Color" (select (Utilities|IsValid (Variables|Default|GetDestinationTeleporter)) (Variables|Default|GetColor) "(R=0.500000,G=0.500000,B=0.500000,A=1.000000)") :!class /Script/Engine.MaterialInstanceDynamic))

(fn CanActorTeleport
  (params (Actor :type Actor%20Object%20Reference))
  (Utilities|Casting|CastToLogHunterCharacter Actor
    (:then
      (return (not (Utilities|Array|ContainsItem (Variables|Default|GetIncomingActors) Actor))))
    (:CastFailed
      (return false))))

(fn HandleIncomingTeleport
  (params (IncomingActor :type Actor%20Object%20Reference) (InvokingTeleport :type Teleporter%20BP%20Object%20Reference))
  (if (not (Utilities|Array|ContainsItem (Variables|Default|GetIncomingActors) IncomingActor))
    (Utilities|Array|Add (Variables|Default|GetIncomingActors) IncomingActor)
    (Transformation|SetActorLocation IncomingActor (+ (Transformation|GetActorLocation IncomingActor) (- (Transformation|GetActorLocation) (Transformation|GetActorLocation InvokingTeleport))) false true)))